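; Hard disk storage task for two spider players: spawns corrupted files to be repaired and collected, then delivered to the compiler.
; The first collecting spider carries files stacked by offset on CubeAnchor, while role-based logs guide both players.
; Server-side checks report pickups and completion to OnlineSession_GM, and EndBox overlap triggers mission completion.
; Finish events activate walkable surfaces, beam FX and screens, then animate the cube into place and raise lighting.
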(event `self.ReceiveBeginPlay`
  (bind _taskwalkablesurface (`self.TaskWalkableSurface`))
  (bind _outactors (`GameplayStatics.GetAllActorsWithTag` "Compilator Screen"))
  (bind _ascompilator_screen_widget (cast `/Game/Scenario/Widgets/CompilatorScreen_Widget` (`WidgetComponent.GetWidget` (`self.GetComponentByClass` (`|GetArrayItem` _outactors) "/Script/UMG.WidgetComponent"))))
  (set `self.EndScreen` _ascompilator_screen_widget)
  (bind _outactors_2 (`GameplayStatics.GetAllActorsWithTag` "StorageState"))
  (bind _ashard_disk_state_widget (cast `/Game/GameplayMechanics/Task/HardDisk/Widgets/HardDiskState_Widget` (`WidgetComponent.GetWidget` (`self.GetComponentByClass` (`|GetArrayItem` _outactors_2) "/Script/UMG.WidgetComponent"))))
  (set `self.StateWidget` _ashard_disk_state_widget)
  (if (`self.begin`)
    (`KismetSystemLibrary.Delay` 2.0)
    (`self.Begin Task`)
    (set `Actor.Tags` (`|MakeArray` "Walkable" :!type "Name") _taskwalkablesurface)
    (bind _asmaterial_instance_dynamic (cast `MaterialInstanceDynamic` (`PrimitiveComponent.GetMaterial` (`StaticMeshActor.StaticMeshComponent` _taskwalkablesurface) 0)))
    (`MaterialInstanceDynamic.SetScalarParameterValue` _asmaterial_instance_dynamic "Activate" 2.0)
    (bind _asmaterial_instance_dynamic_2 (cast `MaterialInstanceDynamic` (`PrimitiveComponent.GetMaterial` (`StaticMeshActor.StaticMeshComponent` (`self.Walkable_3`)) 0)))
    (`MaterialInstanceDynamic.SetScalarParameterValue` _asmaterial_instance_dynamic_2 "Activate" 1.0)))

(event `Spawn File`
  (bind _returnvalue (`|SpawnActorFromClass` "/Game/GameplayMechanics/Task/HardDisk/File/CorruptedFile_BP.CorruptedFile_BP_C" (`KismetMathLibrary.MakeTransform` (+ (`self.K2_GetActorLocation`) (`KismetMathLibrary.MakeVector` (`KismetMathLibrary.RandomFloatInRange` -500.0 500.0) (`KismetMathLibrary.RandomFloatInRange` -500.0 500.0)))) "Undefined" "OverrideRootScale" null null))
  (`KismetArrayLibrary.Array_AddUnique` (`self.files`) _returnvalue)
  (set `/Game/GameplayMechanics/Task/HardDisk/File/CorruptedFile_BP.tasker` self _returnvalue)
  (set `/Game/GameplayMechanics/Task/HardDisk/File/CorruptedFile_BP.index` (`self.CountFiles`) _returnvalue)
  (set `/Game/GameplayMechanics/Task/HardDisk/File/CorruptedFile_BP.offset` (`self.Offset for Cube`) _returnvalue)
  (`/Engine/EditorBlueprintResources/StandardMacros.IncrementInt` (`self.CountFiles`)))

(event `self.Begin Task`
  ;[1 1 1] Init
  (`parent.Begin Task`)
  (`FXSystemComponent.SetVectorParameter` (`self.Niagara`) "Beam End" (`SceneComponent.K2_GetComponentLocation` (`self.EndBox`)))
  (`KismetSystemLibrary.PrintString` "Hello")
  (set `self.cubeShootable` false)
  (set `self.countCubes` 0)
  (`self.Emit FX` false)
  (`KismetArrayLibrary.Array_Clear` (`self.files`))
  ;[1 1 1] Spawn
  (for _ (range 1 (+ (`self.Last Index`) 1))
    (`self.Spawn File`)))

(event `Attach file to spider`
  (params (spider :type "/Game/Spider/Spider_Character Object Reference") (file :type "/Game/GameplayMechanics/Task/HardDisk/File/CorruptedFile_BP Object Reference"))
  (bind _mesh (`Character.Mesh` (`self.spiderWithCube`)))
  (bind _spiderwithcube (`self.spiderWithCube`)
    (:`then`
      (if (== _spiderwithcube spider)
        (set `self.cubeShootable` true)
        (`self.K2_AttachToComponent` file (`self.cubeAnchor`) "None" "SnapToTarget" "SnapToTarget" "KeepRelative" true :!label _label)
        (`/Game/GameplayMechanics/Task/HardDisk/File/CorruptedFile_BP.Reset Location` file)
        (`self.K2_SetActorRelativeLocation` file (`/Game/GameplayMechanics/Task/HardDisk/File/CorruptedFile_BP.offset` file) false false)
        (`/Engine/EditorBlueprintResources/StandardMacros.IncrementInt` (`self.countCubes`)
          (:`  `
            (bind _asonline_session_gm (cast `/Game/Game/OnlineSession_GM` (`GameplayStatics.GetGameMode`)))
            (`/Game/Game/OnlineSession_GM.Update File in UI` _asonline_session_gm (`/Game/GameplayMechanics/Task/HardDisk/File/CorruptedFile_BP.index` file) "collect")
            (`self.Can go to the compilator`)))))
    (:`else`
      (bind _output_get (set `self.spiderWithCube` spider))
      (`SceneComponent.K2_AttachToComponent` (`self.cubeAnchor`) (`Character.Mesh` _output_get) "None" "SnapToTarget" "SnapToTarget" "KeepWorld" true)
      (`SceneComponent.K2_SetRelativeLocation` (`self.cubeAnchor`) (-10.0 0.0 50.0) false false)
      (`SceneComponent.K2_SetWorldRotation` (`self.cubeAnchor`) (`KismetMathLibrary.MakeRotationFromAxes` (`SceneComponent.GetForwardVector` _mesh) (`SceneComponent.GetRightVector` _mesh) (`SceneComponent.GetUpVector` _mesh)) false false)
      (goto _label))))

(event `Can go to the compilator`
  ;[0.4227 0.8939 1] End of the task
  (bind _returnvalue (`self.Check files`))
  (if _returnvalue
    (`/Engine/EditorBlueprintResources/ActorMacros.Switch Has Authority`
      (:`Authority`
        (bind _asonline_session_gm (cast `/Game/Game/OnlineSession_GM` (`GameplayStatics.GetGameMode`)))
        (`/Game/Game/OnlineSession_GM.StockageTaskAccomplished!` _asonline_session_gm)
        (bind (_collecting _rewriting) (`self.Get Spiders`))
        (`/Game/Spider/Spider_Character.Request Log` _collecting "Storage:AllCollected" 0.0)
        (`/Game/Spider/Spider_Character.Request Log` _rewriting "Storage:AllCollected" 0.0)))))

(event `On Finished`
  (bind _walkableend (`self.WalkableEnd`))
  ;[0.4227 0.8939 1] End of the task
  (`KismetSystemLibrary.PrintString` "Suite de l'épreuve" true true (struct :`R` 1.0 :`G` 0.838219 :`A` 1.0))
  (set `Actor.Tags` (`|MakeArray` "Walkable" :!type "Name") _walkableend)
  (bind _asmaterial_instance_dynamic (cast `MaterialInstanceDynamic` (`PrimitiveComponent.GetMaterial` (`StaticMeshActor.StaticMeshComponent` _walkableend) 0)))
  (`MaterialInstanceDynamic.SetScalarParameterValue` _asmaterial_instance_dynamic "Activate" 2.0)
  (`self.Emit FX` true)
  (`/Game/GameplayMechanics/Task/HardDisk/Widgets/HardDiskState_Widget.Complete` (`self.StateWidget`)))

(event `On FInd`
  (bind (_collecting _rewriting) (`self.Get Spiders`))
  (`/Game/Spider/Spider_Character.Request Log` _collecting (`KismetTextLibrary.Conv_StringToText` (`KismetStringLibrary.Concat_StrStr` "One files Extracted : " (`KismetStringLibrary.Conv_IntToString` (- (`self.How Much FIles in state` 0) 1)) " left")) 0.0)
  (`/Game/Spider/Spider_Character.Request Log` _rewriting "Storage:OnReceived" 0.0))

(event `self.EndBox.OnComponentBeginOverlap`
  (params (OverlappedComponent :type "PrimitiveComponent Object Reference") (OtherActor :type "Actor Object Reference") (OtherComp :type "PrimitiveComponent Object Reference") (OtherBodyIndex :type Integer) (bFromSweep :type Boolean) (SweepResult :type "HitResult Structure (by ref)"))
  ;[1 1 1] Collision with endBox
  (if (== OtherActor (`self.spiderWithCube`))
    _
    (else
      _))
  (`/Engine/EditorBlueprintResources/ActorMacros.Switch Has Authority`
    (:`Authority`
      (bind _asonline_session_gm (cast `/Game/Game/OnlineSession_GM` (`GameplayStatics.GetGameMode`)))
      (`/Game/Game/OnlineSession_GM.MissionAccomplissed!!` _asonline_session_gm (`self.rebootCinematic`)))))

(event `On Repaired`
  (bind _collecting (`self.Get Spiders`))
  (`/Game/Spider/Spider_Character.Request Log` _collecting "Storage:FileBack" 0.0)
  (`/Engine/EditorBlueprintResources/StandardMacros.DoOnce` false
    (:`Completed`
      (`/Game/Spider/Spider_Character.Request Message` _collecting "TutoFile:Collect" 8.0))))

(event `S_End`
  ;[1 0.3984 0.4402] End of the game
  (`self.Multcast End`)
  (cast `/Game/Game/Spider_GS` (`GameplayStatics.GetGameState`))
  (set `self.cubeShootable` false)
  (`AudioComponent.Play` (`self.Insert_Audio`) 0.0))

(event `On collected`
  (bind _returnvalue (- (`KismetArrayLibrary.Array_Length` (`self.files`)) (- (`SceneComponent.GetNumChildrenComponents` (`self.cubeAnchor`)) 2)))
  (if (> _returnvalue 0)
    (bind (_collecting _rewriting) (`self.Get Spiders`))
    (`/Game/Spider/Spider_Character.Request Log` _rewriting "Storage:BuddyCollected" 0.0)
    (`/Game/Spider/Spider_Character.Request Log` _collecting (`KismetTextLibrary.Conv_StringToText` (`KismetStringLibrary.Concat_StrStr` "Repaired file collected. \n" (`KismetStringLibrary.Conv_IntToString` _returnvalue) " files left")) 0.0)
    (else
      (bind (_collecting_2 _rewriting_2) (`self.Get Spiders`))
      (`/Game/Spider/Spider_Character.Request Log` _collecting_2 "Storage:AllCollected" 0.0)
      (`/Game/Spider/Spider_Character.Request Log` _rewriting_2 "Storage:AllCollected" 0.0))))

(event `Multcast End`
  ;[1 0.3984 0.4402] End of the game
  (`GameplayStatics.PlaySound2D` "/Engine/VREditor/Sounds/VR_shep_scale_up_02.VR_shep_scale_up_02" 1.0 1.0 0.0 null null)
  (`SceneComponent.K2_DetachFromComponent` (`self.cubeAnchor`) "KeepWorld" "KeepWorld" "KeepWorld" true)
  (bind (_direction _alpha) (`Timeline|SetCube`)
    (:`Update`
      (`SceneComponent.K2_SetWorldLocationAndRotation` (`self.cubeAnchor`) (`KismetMathLibrary.VLerp` (`SceneComponent.K2_GetComponentLocation` (`self.cubeAnchor`)) (`SceneComponent.K2_GetComponentLocation` (`self.EndCubeAnchor`)) _alpha) (`KismetMathLibrary.RLerp` (`SceneComponent.K2_GetComponentRotation` (`self.cubeAnchor`)) (struct :`Roll` 90.0) _alpha) true false))
    (:`Finished`
      (`SceneComponent.K2_SetWorldLocation` (`self.cubeAnchor`) (`SceneComponent.K2_GetComponentLocation` (`self.EndBox`)) true false)
      (`self.Emit FX` false)
      (`PrimitiveComponent.SetCollisionEnabled` (`self.EndBox`) "NoCollision")
      (`/Game/Scenario/Widgets/CompilatorScreen_Widget.Complete` (`self.EndScreen`))
      (bind _asmaterial_instance_dynamic (cast `MaterialInstanceDynamic` (`PrimitiveComponent.GetMaterial` (`StaticMeshActor.StaticMeshComponent` (`self.Walkable_3`)) 0)))
      (`MaterialInstanceDynamic.SetScalarParameterValue` _asmaterial_instance_dynamic "Activate" 2.0)
      (bind _asmaterial_instance_dynamic_2 (cast `MaterialInstanceDynamic` (`PrimitiveComponent.GetMaterial` (`StaticMeshActor.StaticMeshComponent` (`self.Walkable_2`)) 0)))
      (`MaterialInstanceDynamic.SetScalarParameterValue` _asmaterial_instance_dynamic_2 "Activate" 2.0)
      (bind _outactors (`GameplayStatics.GetAllActorsOfClass` "/Script/Engine.RectLight"))
      (for _array_element _outactors
        (`LightComponent.SetIntensity` (`Light.LightComponent` _array_element) (`KismetMathLibrary.SelectFloat` 1000.0 25.0 (`self.ActorHasTag` _array_element "hot")))
        (`KismetSystemLibrary.PrintString` "Hello" :!label _label_2))
      (bind _outactors_2 (`GameplayStatics.GetAllActorsOfClass` "/Script/Engine.SpotLight"))
      (for _array_element_2 _outactors_2
        (if (not (`self.ActorHasTag` _array_element_2 "grid"))
          (`LightComponent.SetIntensity` (`Light.LightComponent` _array_element_2) 1000.0)
          (goto _label_2))))))

(event `self.playBox.OnComponentBeginOverlap`
  (params (OverlappedComponent :type "PrimitiveComponent Object Reference") (OtherActor :type "Actor Object Reference") (OtherComp :type "PrimitiveComponent Object Reference") (OtherBodyIndex :type Integer) (bFromSweep :type Boolean) (SweepResult :type "HitResult Structure (by ref)"))
  (if (`self.has begun`)
    (if (not (!= (`KismetArrayLibrary.Array_Find` (`ActorComponent.ComponentTags` OtherComp) "Karcher") -1))
      (bind _asspider_character (cast `/Game/Spider/Spider_Character` OtherActor))
      (`/Engine/EditorBlueprintResources/ActorMacros.Switch Has Authority`
        (:`Authority`
          (`|ExecutionSequence`
            (:`then_0`
              (bind _asonline_session_gm (cast `/Game/Game/OnlineSession_GM` (`GameplayStatics.GetGameMode`))))
            (:`then_1`
              (if (`self.ActorHasTag` _asspider_character "Player 1")
                (`/Engine/EditorBlueprintResources/StandardMacros.DoOnce` false
                  (:`Completed`
                    (`/Game/Game/OnlineSession_GM.Begin StorageTask` _asonline_session_gm 0)))
                (elif (`self.ActorHasTag` _asspider_character "Player 2")
                  (`/Engine/EditorBlueprintResources/StandardMacros.DoOnce` false
                    (:`Completed`
                      (`/Game/Game/OnlineSession_GM.Begin StorageTask` _asonline_session_gm 1))))))))))))

(event `self.UpBox.OnComponentBeginOverlap`
  (params (OverlappedComponent :type "PrimitiveComponent Object Reference") (OtherActor :type "Actor Object Reference") (OtherComp :type "PrimitiveComponent Object Reference") (OtherBodyIndex :type Integer) (bFromSweep :type Boolean) (SweepResult :type "HitResult Structure (by ref)"))
  (if (`self.has begun`)
    (if (not (!= (`KismetArrayLibrary.Array_Find` (`ActorComponent.ComponentTags` OtherComp) "Karcher") -1))
      (bind _asspider_character (cast `/Game/Spider/Spider_Character` OtherActor))
      (`/Engine/EditorBlueprintResources/StandardMacros.DoOnce` false
        (:`Completed`
          (`/Engine/EditorBlueprintResources/ActorMacros.Switch Has Authority`
            (:`Authority`
              (`/Game/Spider/Spider_Character.Request Log` _asspider_character "Storage:FindFiles" 0.0)
              (`/Game/Spider/Spider_Character.Request Message` _asspider_character "TutoFile:FindFIle" 8.0))))))))

(event `self.DownBox.OnComponentBeginOverlap`
  (params (OverlappedComponent :type "PrimitiveComponent Object Reference") (OtherActor :type "Actor Object Reference") (OtherComp :type "PrimitiveComponent Object Reference") (OtherBodyIndex :type Integer) (bFromSweep :type Boolean) (SweepResult :type "HitResult Structure (by ref)"))
  (if (`self.has begun`)
    (if (not (!= (`KismetArrayLibrary.Array_Find` (`ActorComponent.ComponentTags` OtherComp) "Karcher") -1))
      (bind _asspider_character (cast `/Game/Spider/Spider_Character` OtherActor))
      (`/Engine/EditorBlueprintResources/StandardMacros.DoOnce` false
        (:`Completed`
          (`/Engine/EditorBlueprintResources/ActorMacros.Switch Has Authority`
            (:`Authority`
              (`/Game/Spider/Spider_Character.Request Log` _asspider_character "Storage:Wait" 0.0))))))))

(fn `Check files`
  (returns (ReturnValue :type Boolean))
  (return (== (- (`SceneComponent.GetNumChildrenComponents` (`self.cubeAnchor`)) 1) (`KismetArrayLibrary.Array_Length` (`self.files`)))))

(fn `Emit FX`
  (params (bNewEnableState :type Boolean))
  (if bNewEnableState
    (`ActorComponent.Activate` (`self.Niagara`) false)
    (else
      (`ActorComponent.Deactivate` (`self.Niagara`)))))

(fn `Get Spiders`
  (returns (Collecting :type "/Game/Spider/Spider_Character Object Reference") (Rewriting :type "/Game/Spider/Spider_Character Object Reference"))
  (bind _spiderwithcube (`self.spiderWithCube`))
  (bind _outactors (`GameplayStatics.GetAllActorsOfClass` "/Game/Spider/Spider_Character.Spider_Character_C"))
  (`/Engine/EditorBlueprintResources/StandardMacros.IsValid` _spiderwithcube
    (:`Is Valid`
      (bind _output (`|GetArrayItem` _outactors))
      (bind _output_2 (`|GetArrayItem` _outactors 1))
      (return _spiderwithcube (select `bool` (== _output _spiderwithcube) :`false` _output :`true` _output_2)))
    (:`Is Not Valid`
      (bind (_returnvalue_x _returnvalue_y _returnvalue_z) (`KismetMathLibrary.BreakVector` (`self.K2_GetActorLocation` _output)))
      (bind (_returnvalue_x_2 _returnvalue_y_2 _returnvalue_z_2) (`KismetMathLibrary.BreakVector` (`self.K2_GetActorLocation` _output_2)))
      (bind _returnvalue (> _returnvalue_z _returnvalue_z_2))
      (return (select `bool` _returnvalue :`false` _output_2 :`true` _output) (select `bool` _returnvalue :`false` _output :`true` _output_2)))))

(fn `How Much FIles in state`
  (params (stateID :type Integer))
  (returns (res :type Integer))
  (locals (count :type Integer))
  (set `local.count` 0)
  (for _array_element (`self.files`)
    (if (== (`/Game/GameplayMechanics/Task/HardDisk/File/CorruptedFile_BP.StateID` _array_element) stateID)
      (`/Engine/EditorBlueprintResources/StandardMacros.IncrementInt` (`local.count`))))
  (return (`local.count`)))

(fn `Offset for Cube`
  (returns (Output :type "Vector Structure"))
  (bind _offset (`self.Offset`))
  (bind _offset_2 (`self.Offset`))
  (bind _countfiles (`self.CountFiles`))
  (return (`KismetMathLibrary.MakeVector` (+ (- (* (mod (/ _countfiles 3) 2) _offset_2) _offset) 10.0) (- (* (mod _countfiles 3) _offset_2) _offset) (+ (- (* (/ _countfiles 6) _offset_2) _offset) 10.0))))

(fn `OnRep_countCubes`
  (`KismetSystemLibrary.PrintString` (`KismetStringLibrary.Conv_IntToString` (`self.countCubes`))))

(fn `UserConstructionScript`
  (`parent.UserConstructionScript`))