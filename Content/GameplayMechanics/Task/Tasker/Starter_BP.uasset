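; Starter_BP is a task trigger pad that detects spider characters and can be confirmed to signal a task start.
; Box overlaps, filtered by body-only macros, show or remove the controller's inform widget and update Presence, clearing Confirmed when presence ends.
; Confirm sets Confirmed.
; RepNotifies on both flags swap the plane material between idle, occupied and confirmed, and Confirmed's notify also fires OnConfirm.
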(event `self.Box.OnComponentBeginOverlap`
  (params (OverlappedComponent :type "PrimitiveComponent Object Reference") (OtherActor :type "Actor Object Reference") (OtherComp :type "PrimitiveComponent Object Reference") (OtherBodyIndex :type Integer) (bFromSweep :type Boolean) (SweepResult :type "HitResult Structure (by ref)"))
  ;[0.4355 0.5579 0.9302] Widget
  (bind _asspider_character (cast `/Game/Spider/Spider_Character` OtherActor))
  (if (not (or (== _asspider_character (`/Game/Spider/Spider_Character.TaserTarget` _asspider_character)) (== _asspider_character (`/Game/Spider/Spider_Character.KarcherTarget` _asspider_character))))
    (bind _asspider_bots_controller (cast `/Game/Game/SpiderBots_Controller` (`Pawn.GetController` _asspider_character)))
    (`/Game/Game/SpiderBots_Controller.Display Inform Widget` _asspider_bots_controller (`self.task them`))
    (set `self.presence` true)))

(event `self.Box.OnComponentEndOverlap`
  (params (OverlappedComponent :type "PrimitiveComponent Object Reference") (OtherActor :type "Actor Object Reference") (OtherComp :type "PrimitiveComponent Object Reference") (OtherBodyIndex :type Integer))
  ;[0.4355 0.5579 0.9302] Widget
  (bind _asspider_character (cast `/Game/Spider/Spider_Character` OtherActor))
  (if (not (or (== _asspider_character (`/Game/Spider/Spider_Character.TaserTarget` _asspider_character)) (== _asspider_character (`/Game/Spider/Spider_Character.KarcherTarget` _asspider_character))))
    (bind _asspider_bots_controller (cast `/Game/Game/SpiderBots_Controller` (`Pawn.GetController` _asspider_character)))
    (`/Game/Game/SpiderBots_Controller.Remove Inform Widget` _asspider_bots_controller)
    (bind _output_get (set `self.presence` (> (`KismetArrayLibrary.Array_Length` (`PrimitiveComponent.GetOverlappingActors` (`self.Plane`) "/Game/Spider/Spider_Character.Spider_Character_C")) 1)))
    (if (not _output_get)
      (set `self.confirmed` false))))

(event `Plane Mat Rep _ Server`
  (bind _plane (`self.Plane`))
  ;[0.3 0.0411 0.0411] Replication
  (if (`self.confirmed`)
    (`PrimitiveComponent.SetMaterial` (`self.Plane`) 0 "/Game/GameplayMechanics/Taser/Board/target_Mat_Inst.target_Mat_Inst")
    (elif (`self.presence`)
      (`PrimitiveComponent.SetMaterial` _plane 0 "/Engine/EngineMaterials/CubeMaterial.CubeMaterial")
      (else
        (`PrimitiveComponent.SetMaterial` _plane 0 "/Engine/BasicShapes/BasicShapeMaterial.BasicShapeMaterial")))))

(event `Confirm`
  (if (not (`self.confirmed`))
    (set `self.confirmed` true)))

(event `C_ Confirm`
  (`self.Confirm`))

(fn `OnRep_confirmed`
  (`self.Plane Mat Rep _ Server`)
  (`self.OnConfirm`))

(fn `OnRep_presence`
  (`self.Plane Mat Rep _ Server`))

(fn `UserConstructionScript`)