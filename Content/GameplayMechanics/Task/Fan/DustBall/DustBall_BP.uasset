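; Dust ball for the fan/blower task that players clean with the Karcher tool.
; On the server, sphere overlaps with Karcher-tagged components start and end shots on its ShootableComponent through Spider_GS, toggling the dust effect's visibility.
; The component's OnShot event clears Interactable, whose RepNotify updates collision and the BlowerTask_BP widget on authority, then calls MC_Clean to update Niagara and hide the dust ball's widget.
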(event `MC_Clean`
  (if (`self.interactable`)
    (`ActorComponent.Activate` (`self.Niagara`) false)
    (else
      (`ActorComponent.Deactivate` (`self.Niagara`))
      (`SceneComponent.SetVisibility` (`self.Widget`) false false)))
  (bind _asdust_ball_widget (cast `/Game/GameplayMechanics/Task/Fan/DustBall/DustBall_Widget` (`WidgetComponent.GetWidget` (`self.Widget`))))
  (`/Game/GameplayMechanics/Task/Fan/DustBall/DustBall_Widget.Hide` _asdust_ball_widget))

(event `self.ReceiveBeginPlay`
  (add `/Game/GameplayMechanics/Karcher/Shootable_Component.OnShot` (`self.Shootable_Component`) (delegate `Clean`)))

(event `Clean`
  (set `self.interactable` false))

(event `self.Sphere.OnComponentBeginOverlap`
  (params (OverlappedComponent :type "PrimitiveComponent Object Reference") (OtherActor :type "Actor Object Reference") (OtherComp :type "PrimitiveComponent Object Reference") (OtherBodyIndex :type Integer) (bFromSweep :type Boolean) (SweepResult :type "HitResult Structure (by ref)"))
  (`/Engine/EditorBlueprintResources/ActorMacros.Switch Has Authority`
    (:`Authority`
      (if (!= (`KismetArrayLibrary.Array_Find` (`ActorComponent.ComponentTags` OtherComp) "Karcher") -1)
        (bind _asspider_gs (cast `/Game/Game/Spider_GS` (`GameplayStatics.GetGameState`)))
        (`/Game/Game/Spider_GS.Karcher shot OnServer` _asspider_gs (`self.Shootable_Component`) (`KismetMathLibrary.GetDirectionUnitVector` (`self.K2_GetActorLocation` OtherActor) (`self.K2_GetActorLocation`)))
        (`SceneComponent.SetVisibility` (`self.Niagara`) false false)))))

(event `self.Sphere.OnComponentEndOverlap`
  (params (OverlappedComponent :type "PrimitiveComponent Object Reference") (OtherActor :type "Actor Object Reference") (OtherComp :type "PrimitiveComponent Object Reference") (OtherBodyIndex :type Integer))
  (`/Engine/EditorBlueprintResources/ActorMacros.Switch Has Authority`
    (:`Authority`
      (if (!= (`KismetArrayLibrary.Array_Find` (`ActorComponent.ComponentTags` OtherComp) "Karcher") -1)
        (bind _asspider_gs (cast `/Game/Game/Spider_GS` (`GameplayStatics.GetGameState`)))
        (`/Game/Game/Spider_GS.Karcher shot OnServer` _asspider_gs (`self.Shootable_Component`) (0.0 0.0 0.0))
        (`SceneComponent.SetVisibility` (`self.Niagara`) (`self.interactable`) false)))))

(fn `Get Is Clean`
  (returns (isClean :type Boolean))
  (return (< (`/Game/GameplayMechanics/Karcher/Shootable_Component.Resistance` (`self.Shootable_Component`)) 0.0)))

(fn `OnRep_interactable`
  (`/Engine/EditorBlueprintResources/ActorMacros.Switch Has Authority`
    (:`Authority`
      (`PrimitiveComponent.SetCollisionEnabled` (`self.Sphere`) (select `bool` (`self.interactable`) :`false` "NoCollision" :`true` "QueryOnly" :!type "ECollisionEnabled Enum"))
      (`|ExecutionSequence`
        (:`then_0`
          (bind _returnvalue (`GameplayStatics.GetActorOfClass` "/Game/GameplayMechanics/Task/Fan/BlowerTask_BP.BlowerTask_BP_C"))
          (`/Game/GameplayMechanics/Task/Fan/BlowerTask_BP.S_Update Blower Widget` _returnvalue))
        (:`then_1`
          (`self.MC_Clean`))))))

(fn `UserConstructionScript`)