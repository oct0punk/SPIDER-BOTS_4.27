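; Tasker blueprint that begins a gameplay task once both of its starters are confirmed.
; TestEvent checks the Confirmed state of Starter1 and Starter2, hides both starters when both are set, then calls BeginTask.
; BeginTask sets HasBegun, and ServerTest simply forwards to TestEvent.
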(event `TestEvent`
  (if (and (`/Game/GameplayMechanics/Task/Starter_BP.confirmed` (`self.starter1`)) (`/Game/GameplayMechanics/Task/Starter_BP.confirmed` (`self.starter2`)))
    (`/Game/GameplayMechanics/Task/Starter_BP.Hide starter` (`self.starter1`))
    (`/Game/GameplayMechanics/Task/Starter_BP.Hide starter` (`self.starter2`))
    (`self.Begin Task`)))

(event `Server Test`
  (`self.TestEvent`))

(event `Begin Task`
  (set `self.has begun` true))

(fn `UserConstructionScript`)