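; Taser target board that a Spider character activates by overlapping its box with a component tagged "Taser".
; On authority, that overlap records the spider and has the game state trigger the TasableComponent; other spider overlaps request a taser intro log.
; The component's OnTased event plays audio and sets the plane's dynamic material emission and rect light intensity from its Active state.
; The widget starts hidden and is hidden again on end overlap.
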(event `self.ReceiveBeginPlay`
  (add `/Game/GameplayMechanics/Taser/Tasable_Component.On Tased` (`self.Tasable_Component`) (delegate `Change Plane's Mat`))
  (`SceneComponent.SetVisibility` (`self.Widget`) false false)
  (bind _returnvalue (`PrimitiveComponent.CreateDynamicMaterialInstance` (`self.Plane`) 0 "/Game/GameplayMechanics/Taser/Board/target_Mat_Inst.target_Mat_Inst" "None"))
  (`PrimitiveComponent.SetMaterial` (`self.Plane`) 0 _returnvalue))

(event `Change Plane's Mat`
  (bind _returnvalue (`KismetMathLibrary.Conv_BoolToInt` (`/Game/GameplayMechanics/Taser/Tasable_Component.Active` (`self.Tasable_Component`))))
  (`AudioComponent.Play` (`self.Audio`) 0.0)
  (bind _asmaterial_instance_dynamic (cast `MaterialInstanceDynamic` (`PrimitiveComponent.GetMaterial` (`self.Plane`) 0)))
  (`MaterialInstanceDynamic.SetScalarParameterValue` _asmaterial_instance_dynamic "emission" (* _returnvalue 3.0))
  (`LightComponent.SetIntensity` (`self.RectLight`) (* _returnvalue 3000.0)))

(event `self.Box.OnComponentBeginOverlap`
  (params (OverlappedComponent :type "PrimitiveComponent Object Reference") (OtherActor :type "Actor Object Reference") (OtherComp :type "PrimitiveComponent Object Reference") (OtherBodyIndex :type Integer) (bFromSweep :type Boolean) (SweepResult :type "HitResult Structure (by ref)"))
  ;[1 0.628 0.1573] Spider use "taser" on this
  (`/Engine/EditorBlueprintResources/ActorMacros.Switch Has Authority`
    (:`Authority`
      (bind _asspider_character (cast `/Game/Spider/Spider_Character` OtherActor))
      (if (!= (`KismetArrayLibrary.Array_Find` (`ActorComponent.ComponentTags` OtherComp) "Taser") -1)
        (set `self.last spider has tased` _asspider_character)
        (bind _asspider_gs (cast `/Game/Game/Spider_GS` (`GameplayStatics.GetGameState`)))
        (`/Game/Game/Spider_GS.Trigger On Server` _asspider_gs (`self.Tasable_Component`))
        (else
          (`/Game/Spider/Spider_Character.Request Log` _asspider_character "Intro:Tazer" 0.0))))))

(event `self.Box.OnComponentEndOverlap`
  (params (OverlappedComponent :type "PrimitiveComponent Object Reference") (OtherActor :type "Actor Object Reference") (OtherComp :type "PrimitiveComponent Object Reference") (OtherBodyIndex :type Integer))
  (bind _asspider_character (cast `/Game/Spider/Spider_Character` OtherActor))
  (`/Game/Spider/Spider_Character.Display tasable widget` _asspider_character (`self.Widget`) false))

(fn `UserConstructionScript`)