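; Target actor that the spider can tase, showing its TasableComponent's active state by swapping the material on a plane.
; A box overlap with a "Taser"-tagged component asks Spider_GS to trigger the TasableComponent on the server, and the OnTased event updates the material.
; Overlap also clears the switcher widget's display flag, and end overlap hides it through Spider_Character.
; The graph that would show the widget is never called.
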(event `self.ReceiveBeginPlay`
  (add `/Game/GameplayMechanics/Taser/Tasable_Component.On Tased` (`self.Tasable_Component`) (delegate `Change Plane's Mat`))
  (`SceneComponent.SetVisibility` (`self.Widget`) false false))

(event `Change Plane's Mat`
  (`PrimitiveComponent.SetMaterial` (`self.Plane`) 0 (select `bool` (`/Game/GameplayMechanics/Taser/Tasable_Component.Active` (`self.Tasable_Component`)) :`false` "/Engine/MapTemplates/Materials/BasicAsset01.BasicAsset01" :`true` "/Engine/MapTemplates/Materials/BasicAsset03.BasicAsset03" :!type "MaterialInterface Object Reference")))

(event `self.Box.OnComponentBeginOverlap`
  (params (OverlappedComponent :type "PrimitiveComponent Object Reference") (OtherActor :type "Actor Object Reference") (OtherComp :type "PrimitiveComponent Object Reference") (OtherBodyIndex :type Integer) (bFromSweep :type Boolean) (SweepResult :type "HitResult Structure (by ref)"))
  ;[1 0.628 0.1573] Spider use "taser" on this
  (`|ExecutionSequence`
    (:`then_0`
      (bind _asswitcher_widget (cast `/Game/GameplayMechanics/Taser/Switcher_Widget` (`WidgetComponent.GetWidget` (`self.Widget`))))
      (set `/Game/GameplayMechanics/Taser/Switcher_Widget.should display` false _asswitcher_widget))
    (:`then_1`
      (if (!= (`KismetArrayLibrary.Array_Find` (`ActorComponent.ComponentTags` OtherComp) "Taser") -1)
        (bind _asspider_gs (cast `/Game/Game/Spider_GS` (`GameplayStatics.GetGameState`)))
        (`/Game/Game/Spider_GS.Trigger On Server` _asspider_gs (`self.Tasable_Component`))))))

(event `self.Box.OnComponentEndOverlap`
  (params (OverlappedComponent :type "PrimitiveComponent Object Reference") (OtherActor :type "Actor Object Reference") (OtherComp :type "PrimitiveComponent Object Reference") (OtherBodyIndex :type Integer))
  (bind _asspider_character (cast `/Game/Spider/Spider_Character` OtherActor))
  (`/Game/Spider/Spider_Character.Display tasable widget` _asspider_character (`self.Widget`) false))

(fn `UserConstructionScript`)