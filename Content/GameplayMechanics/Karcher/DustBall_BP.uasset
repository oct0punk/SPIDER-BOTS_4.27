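; DustBall_BP is a dust ball that is cleaned with the Karcher tool.
; Overlaps with Karcher-tagged components send the ShootableComponent and a push direction away from the overlapping actor to Spider_GS.KarcherShotOnServer, with a zero direction on exit.
; The component's shot event clears Interactable, whose RepNotify updates sphere collision and visibility and refreshes the game mode's blower widget.
; GetIsClean reports whether the component's Resistance has dropped below zero.
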(event `self.ReceiveBeginPlay`
  (add `/Game/GameplayMechanics/Karcher/Shootable_Component.OnShot` (`self.Shootable_Component`) (delegate `Clean`)))

(event `Clean`
  (set `self.interactable` false))

(event `self.Sphere.OnComponentBeginOverlap`
  (params (OverlappedComponent :type "PrimitiveComponent Object Reference") (OtherActor :type "Actor Object Reference") (OtherComp :type "PrimitiveComponent Object Reference") (OtherBodyIndex :type Integer) (bFromSweep :type Boolean) (SweepResult :type "HitResult Structure (by ref)"))
  (if (!= (`KismetArrayLibrary.Array_Find` (`ActorComponent.ComponentTags` OtherComp) "Karcher") -1)
    (bind _asspider_gs (cast `/Game/Game/Spider_GS` (`GameplayStatics.GetGameState`)))
    (`/Game/Game/Spider_GS.Karcher shot OnServer` _asspider_gs (`self.Shootable_Component`) (`KismetMathLibrary.GetDirectionUnitVector` (`self.K2_GetActorLocation` OtherActor) (`self.K2_GetActorLocation`)))))

(event `self.Sphere.OnComponentEndOverlap`
  (params (OverlappedComponent :type "PrimitiveComponent Object Reference") (OtherActor :type "Actor Object Reference") (OtherComp :type "PrimitiveComponent Object Reference") (OtherBodyIndex :type Integer))
  (if (!= (`KismetArrayLibrary.Array_Find` (`ActorComponent.ComponentTags` OtherComp) "Karcher") -1)
    (bind _asspider_gs (cast `/Game/Game/Spider_GS` (`GameplayStatics.GetGameState`)))
    (`/Game/Game/Spider_GS.Karcher shot OnServer` _asspider_gs (`self.Shootable_Component`) (0.0 0.0 0.0))))

(fn `Get Is Clean`
  (returns (isClean :type Boolean))
  (return (< (`/Game/GameplayMechanics/Karcher/Shootable_Component.Resistance` (`self.Shootable_Component`)) 0.0)))

(fn `OnRep_interactable`
  (`PrimitiveComponent.SetCollisionEnabled` (`self.Sphere`) (select `bool` (`self.interactable`) :`false` "NoCollision" :`true` "QueryOnly" :!type "ECollisionEnabled Enum"))
  (`SceneComponent.SetVisibility` (`self.Sphere`) (`self.interactable`) false)
  (bind _asonline_session_gm (cast `/Game/Game/OnlineSession_GM` (`GameplayStatics.GetGameMode`)))
  (`/Game/Game/OnlineSession_GM.Update Blower Widget` _asonline_session_gm))

(fn `UserConstructionScript`)