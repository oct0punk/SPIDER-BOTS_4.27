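; Storage task actor for an online spider game, where corrupted files are collected and carried to an end box.
; BeginTask opens the walkable surface and spawns files, which attach to a single spider's CubeAnchor in stacked 3x3 layers.
; Authority notifies OnlineSession_GM of task completion and of the carrier reaching EndBox.
; OnFinished opens the exit surface and Niagara beam, while S_End sends the stack into the box via timeline.
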(event `self.ReceiveBeginPlay`)

(event `Spawn File`
  (bind _returnvalue (`|SpawnActorFromClass` "/Game/Machine/Stockage/CorruptedFile_BP.CorruptedFile_BP_C" (`KismetMathLibrary.MakeTransform` (+ (`self.K2_GetActorLocation`) (`KismetMathLibrary.MakeVector` (`KismetMathLibrary.RandomFloatInRange` -500.0 500.0) (`KismetMathLibrary.RandomFloatInRange` -500.0 500.0)))) "Undefined" "OverrideRootScale" null null))
  (`KismetArrayLibrary.Array_AddUnique` (`self.files`) _returnvalue)
  (set `/Game/Machine/Stockage/CorruptedFile_BP.tasker` self _returnvalue)
  (set `/Game/Machine/Stockage/CorruptedFile_BP.index` (`self.CountFiles`) _returnvalue)
  (`/Engine/EditorBlueprintResources/StandardMacros.IncrementInt` (`self.CountFiles`)))

(event `self.Begin Task`
  (bind _taskwalkablesurface (`self.TaskWalkableSurface`))
  (`FXSystemComponent.SetVectorParameter` (`self.Niagara`) "Beam End" (`SceneComponent.K2_GetComponentLocation` (`self.EndBox`)))
  (`KismetSystemLibrary.PrintString` "Storage Task")
  (`/Engine/EditorBlueprintResources/ActorMacros.Switch Has Authority`
    (:`Authority`
      (bind _asonline_session_gm (cast `/Game/Game/OnlineSession_GM` (`GameplayStatics.GetGameMode`)))
      (`/Game/Game/OnlineSession_GM.Begin StorageTask` _asonline_session_gm))
    (:`Remote`
      _))
  ;[1 1 1] Init
  (set `self.cubeShootable` false)
  (set `self.countCubes` 0)
  (`self.Emit FX` false)
  (`KismetArrayLibrary.Array_Clear` (`self.files`))
  (set `Actor.Tags` (`|MakeArray` "Walkable" :!type "Name") _taskwalkablesurface)
  (bind _asmaterial_instance_dynamic (cast `MaterialInstanceDynamic` (`PrimitiveComponent.GetMaterial` (`StaticMeshActor.StaticMeshComponent` _taskwalkablesurface) 0)))
  (`MaterialInstanceDynamic.SetVectorParameterValue` _asmaterial_instance_dynamic "Grid Color" (struct :`G` 0.363921 :`B` 0.4 :`A` 1.0))
  ;[1 1 1] Spawn
  (for _ (range 1 (+ (`self.Last Index`) 1))
    (`self.Spawn File`)))

(event `Attach file to spider`
  (params (spider :type "/Game/Spider/Spider_Character Object Reference") (file :type "/Game/Machine/Stockage/CorruptedFile_BP Object Reference"))
  (bind _spiderwithcube (`self.spiderWithCube`)
    (:`then`
      (if (== _spiderwithcube spider)
        (set `self.cubeShootable` true)
        (`self.K2_AttachToComponent` file (`self.cubeAnchor`) "None" "SnapToTarget" "SnapToTarget" "KeepRelative" true :!label _label)
        (`/Game/Machine/Stockage/CorruptedFile_BP.Reset Location` file)
        (`self.K2_SetActorRelativeLocation` file (`self.Offset for Cube`) false false)
        (`/Engine/EditorBlueprintResources/StandardMacros.IncrementInt` (`self.countCubes`)
          (:`  `
            (bind _asonline_session_gm (cast `/Game/Game/OnlineSession_GM` (`GameplayStatics.GetGameMode`)))
            (`/Game/Game/OnlineSession_GM.Update File in UI` _asonline_session_gm (`/Game/Machine/Stockage/CorruptedFile_BP.index` file) "collect")
            (`self.Can go to the compilator`)))))
    (:`else`
      (bind _output_get (set `self.spiderWithCube` spider))
      (`SceneComponent.K2_AttachToComponent` (`self.cubeAnchor`) (`Character.Mesh` _output_get) "None" "SnapToTarget" "SnapToTarget" "KeepWorld" true)
      (`SceneComponent.K2_SetRelativeLocation` (`self.cubeAnchor`) (0.0 0.0 120.0) false false)
      (goto _label))))

(event `Can go to the compilator`
  ;[0.4227 0.8939 1] End of the task
  (bind _returnvalue (`self.Check files`))
  (if _returnvalue
    (`/Engine/EditorBlueprintResources/ActorMacros.Switch Has Authority`
      (:`Authority`
        (bind _asonline_session_gm (cast `/Game/Game/OnlineSession_GM` (`GameplayStatics.GetGameMode`)))
        (`/Game/Game/OnlineSession_GM.StockageTaskAccomplished!` _asonline_session_gm)))))

(event `On Finished`
  (bind _walkableend (`self.WalkableEnd`))
  ;[0.4227 0.8939 1] End of the task
  (`KismetSystemLibrary.PrintString` "Suite de l'épreuve" true true (struct :`R` 1.0 :`G` 0.838219 :`A` 1.0))
  (set `Actor.Tags` (`|MakeArray` "Walkable" :!type "Name") _walkableend)
  (bind _asmaterial_instance_dynamic (cast `MaterialInstanceDynamic` (`PrimitiveComponent.GetMaterial` (`StaticMeshActor.StaticMeshComponent` _walkableend) 0)))
  (`MaterialInstanceDynamic.SetVectorParameterValue` _asmaterial_instance_dynamic "Grid Color" (struct :`G` 0.363921 :`B` 0.4 :`A` 1.0))
  (`self.Emit FX` true))

(event `self.EndBox.OnComponentBeginOverlap`
  (params (OverlappedComponent :type "PrimitiveComponent Object Reference") (OtherActor :type "Actor Object Reference") (OtherComp :type "PrimitiveComponent Object Reference") (OtherBodyIndex :type Integer) (bFromSweep :type Boolean) (SweepResult :type "HitResult Structure (by ref)"))
  ;[1 1 1] Collision with endBox
  (if (== OtherActor (`self.spiderWithCube`))
    (`/Engine/EditorBlueprintResources/ActorMacros.Switch Has Authority`
      (:`Authority`
        (bind _asonline_session_gm (cast `/Game/Game/OnlineSession_GM` (`GameplayStatics.GetGameMode`)))
        (`/Game/Game/OnlineSession_GM.MissionAccomplissed!!` _asonline_session_gm (`self.rebootCinematic`))))))

(event `S_End`
  ;[1 0.3984 0.4402] End of the game
  (`self.Multcast End`)
  (cast `/Game/Game/Spider_GS` (`GameplayStatics.GetGameState`))
  (set `self.cubeShootable` false)
  (`AudioComponent.Play` (`self.Insert_Audio`) 0.0))

(event `Multcast End`
  ;[1 0.3984 0.4402] End of the game
  (`GameplayStatics.PlaySound2D` "/Engine/VREditor/Sounds/VR_shep_scale_up_02.VR_shep_scale_up_02" 1.0 1.0 0.0 null null)
  (`SceneComponent.K2_DetachFromComponent` (`self.cubeAnchor`) "KeepWorld" "KeepWorld" "KeepWorld" true)
  (bind (_direction _alpha) (`Timeline|SetCube`)
    (:`Update`
      (`SceneComponent.K2_SetWorldLocation` (`self.cubeAnchor`) (`KismetMathLibrary.VLerp` (`SceneComponent.K2_GetComponentLocation` (`self.cubeAnchor`)) (`SceneComponent.K2_GetComponentLocation` (`self.EndBox`)) _alpha) true false))
    (:`Finished`
      (`SceneComponent.K2_SetWorldLocation` (`self.cubeAnchor`) (`SceneComponent.K2_GetComponentLocation` (`self.EndBox`)) true false)
      (`self.Emit FX` false)
      (`PrimitiveComponent.SetCollisionEnabled` (`self.EndBox`) "NoCollision"))))

(fn `Check files`
  (returns (ReturnValue :type Boolean))
  (return (== (- (`SceneComponent.GetNumChildrenComponents` (`self.cubeAnchor`)) 1) (`KismetArrayLibrary.Array_Length` (`self.files`)))))

(fn `Emit FX`
  (params (bNewEnableState :type Boolean))
  (if bNewEnableState
    (`ActorComponent.Activate` (`self.Niagara`) false)
    (else
      (`ActorComponent.Deactivate` (`self.Niagara`)))))

(fn `Offset for Cube`
  (returns (Output :type "Vector Structure"))
  (bind _countcubes (`self.countCubes`))
  (bind _offset (`self.Offset`))
  (bind _offset_2 (`self.Offset`))
  (bind _returnvalue (mod _countcubes 9))
  (return (`KismetMathLibrary.MakeVector` (- (* (mod _returnvalue 3) _offset_2) _offset) (- (* (/ _returnvalue 3) _offset_2) _offset) (- (* (/ _countcubes 9) _offset_2) _offset))))

(fn `OnRep_countCubes`
  (`KismetSystemLibrary.PrintString` (`KismetStringLibrary.Conv_IntToString` (`self.countCubes`))))

(fn `UserConstructionScript`
  (`parent.UserConstructionScript`))