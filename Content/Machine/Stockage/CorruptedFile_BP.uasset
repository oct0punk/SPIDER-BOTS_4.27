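; Corrupted file pickup that spiders find by tasing, repair, then carry once clean.
; Taser overlaps start tases through the GameState; finding reveals the cube and slides it between Start and End, swapped after each move.
; Repair uses a gamepad QTE or resistance-based tasing, with light color showing progress.
; Once-only server-style events report found and repaired states to the GameMode UI; touching the clean file attaches it via Tasker.
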(event `self.SphereCollision.OnComponentBeginOverlap`
  (params (OverlappedComponent :type "PrimitiveComponent Object Reference") (OtherActor :type "Actor Object Reference") (OtherComp :type "PrimitiveComponent Object Reference") (OtherBodyIndex :type Integer) (bFromSweep :type Boolean) (SweepResult :type "HitResult Structure (by ref)"))
  ;[0.9052 0.4665 0.08608] On Tased
  (if (`self.clean`)
    (bind _asspider_character (cast `/Game/Spider/Spider_Character` OtherActor))
    (`PrimitiveComponent.SetCollisionEnabled` (`self.SphereCollision`) "NoCollision")
    (`/Game/Machine/Stockage/StockageTask_BP.Attach file to spider` (`self.tasker`) _asspider_character self)
    (elif (!= (`KismetArrayLibrary.Array_Find` (`ActorComponent.ComponentTags` OtherComp) "taser") -1)
      (bind _asspider_character_2 (cast `/Game/Spider/Spider_Character` (`ActorComponent.GetOwner` OtherComp)))
      (set `self.Last spider has tased` _asspider_character_2)
      (bind _asspider_gs (cast `/Game/Game/Spider_GS` (`GameplayStatics.GetGameState`)))
      (`/Game/Game/Spider_GS.Begin Tase` _asspider_gs (`self.Tasable_Component`) true))))

(event `self.SphereCollision.OnComponentEndOverlap`
  (params (OverlappedComponent :type "PrimitiveComponent Object Reference") (OtherActor :type "Actor Object Reference") (OtherComp :type "PrimitiveComponent Object Reference") (OtherBodyIndex :type Integer))
  ;[0.9052 0.4665 0.08608] On Tased
  (if (!= (`KismetArrayLibrary.Array_Find` (`ActorComponent.ComponentTags` OtherComp) "taser") -1)
    (bind _asspider_gs (cast `/Game/Game/Spider_GS` (`GameplayStatics.GetGameState`)))
    (`/Game/Game/Spider_GS.Begin Tase` _asspider_gs (`self.Tasable_Component`) false)))

(event `Emit FX`
  ;[1 1 1] FX
  (`ActorComponent.Activate` (`self.ParticleSystem`) true)
  (`FXSystemComponent.SetEmitterEnable` (`self.ParticleSystem`) "Particle Emitter" true))

(event `Move`
  ;[1 1 1] Move
  (`PrimitiveComponent.SetCollisionEnabled` (`self.SphereCollision`) "NoCollision")
  (`/Game/Spider/Spider_Character.No vibrations` (`self.Last spider has tased`))
  (bind (_direction _lerp_s_alpha) (`Timeline|Move Curve` :!via `PlayFromStart`)
    (:`Update`
      (`SceneComponent.K2_SetWorldLocationAndRotation` (`self.Cube`) (`KismetMathLibrary.VLerp` (`SceneComponent.K2_GetComponentLocation` (`self.Start`)) (`SceneComponent.K2_GetComponentLocation` (`self.End`)) _lerp_s_alpha) (`KismetMathLibrary.RLerp` (`SceneComponent.K2_GetComponentRotation` (`self.Start`)) (`SceneComponent.K2_GetComponentRotation` (`self.End`)) _lerp_s_alpha) false false))
    (:`Finished`
      (`self.Swap Start & End`)
      (`PrimitiveComponent.SetCollisionEnabled` (`self.SphereCollision`) "QueryOnly")
      (`SceneComponent.SetVisibility` (`self.Widget`) false false))))

(event `Emit No FX`
  ;[1 1 1] FX
  (`FXSystemComponent.SetEmitterEnable` (`self.ParticleSystem`) "Particle Emitter" false))

(event `self.ReceiveBeginPlay`
  (add `/Game/GameplayMechanics/Taser/Tasable_Component.On Tased` (`self.Tasable_Component`) (delegate `Find`))
  (`self.Emit No FX`)
  (`SceneComponent.SetVisibility` (`self.Cube`) false false)
  (`SceneComponent.SetVisibility` (`self.Widget`) false false)
  (set `self.leftErrors` (`KismetMathLibrary.RandomIntegerInRange` 1 3))
  (set `self.rightErrors` (`KismetMathLibrary.RandomIntegerInRange` 1 3))
  (set `/Game/GameplayMechanics/Taser/Tasable_Component.Resistance` 0.6 (`self.Tasable_Component`)))

(event `Find`
  (`self.S_Find`))

(event `S_Find`
  (bind _tasable_component (`self.Tasable_Component`))
  (`/Engine/EditorBlueprintResources/StandardMacros.DoOnce` false
    (:`Completed`
      (`KismetSystemLibrary.PrintString` "Found" true true (struct :`R` 0.6625 :`G` 0.055208 :`B` 0.055208 :`A` 1.0))
      (`SceneComponent.SetVisibility` (`self.Cube`) true true)
      (`self.Move`)
      (`SceneComponent.SetVisibility` (`self.Widget`) false false)
      (set `/Game/GameplayMechanics/Taser/Tasable_Component.Resistance` 1.5 (`self.Tasable_Component`))
      (clear `/Game/GameplayMechanics/Taser/Tasable_Component.On Tased` _tasable_component)
      (clear `/Game/GameplayMechanics/Taser/Tasable_Component.On Begin Tase` _tasable_component)
      (clear `/Game/GameplayMechanics/Taser/Tasable_Component.On End Tase` _tasable_component)
      (add `/Game/GameplayMechanics/Taser/Tasable_Component.On Begin Tase` _tasable_component (`|CreateDelegate` :!event `Repair task`))
      (bind _asonline_session_gm (cast `/Game/Game/OnlineSession_GM` (`GameplayStatics.GetGameMode`)))
      (`/Game/Game/OnlineSession_GM.Update File in UI` _asonline_session_gm (`self.index`) "found"))))

(event `Repair task`
  (if (`/Game/Spider/Spider_Character.get is gamepad` (`self.Last spider has tased`))
    (`self.QTE Time`)
    (else
      (`self.No QTE`))))

(event `No QTE Repairing`
  (`LightComponent.SetLightColor` (`self.PointLight`) (`KismetMathLibrary.LinearColorLerp` (struct :`R` 0.267366 :`G` 0.908333 :`A` 1.0) (struct :`R` 0.933333 :`G` 0.036518 :`A` 1.0) (`KismetMathLibrary.NormalizeToRange` (`/Game/GameplayMechanics/Taser/Tasable_Component.Resistance` (`self.Tasable_Component`)) 0.0 1.4)) true))

(event `QTE Time`
  ;[1 1 1] QTE
  (`KismetSystemLibrary.PrintString` "QTE" true true (struct :`R` 0.999114 :`G` 1.0 :`B` 0.269225 :`A` 1.0) 3.0)
  (`/Game/Spider/Spider_Character.QTE State` (`self.Last spider has tased`) self)
  (`self.Emit FX`))

(event `M_On Data Repaired`
  ;[1 1 1] QTE
  (`LightComponent.SetLightColor` (`self.PointLight`) (`KismetMathLibrary.LinearColorLerp` (struct :`R` 0.267366 :`G` 0.908333 :`A` 1.0) (struct :`R` 0.933333 :`G` 0.036518 :`A` 1.0) (`self.get errors alpha`)) true))

(event `No QTE`
  (set `/Game/GameplayMechanics/Taser/Tasable_Component.Resistance` 1.4 (`self.Tasable_Component`))
  (add `/Game/GameplayMechanics/Taser/Tasable_Component.On Begin Tase` (`self.Tasable_Component`) (`|CreateDelegate` :!event `Emit FX`))
  (add `/Game/GameplayMechanics/Taser/Tasable_Component.On End Tase` (`self.Tasable_Component`) (`|CreateDelegate` :!event `Emit No FX`))
  (add `/Game/GameplayMechanics/Taser/Tasable_Component.On Tasing` (`self.Tasable_Component`) (`|CreateDelegate` :!event `No QTE Repairing`))
  (add `/Game/GameplayMechanics/Taser/Tasable_Component.On Tased` (`self.Tasable_Component`) (`|CreateDelegate` :!event `S_On repaired`))
  (`self.Emit FX`))

(event `S_On Data Repaired`
  ;[1 1 1] QTE
  (`self.M_On Data Repaired`))

(event `S_On repaired`
  (`/Engine/EditorBlueprintResources/StandardMacros.DoOnce` false
    (:`Completed`
      (`KismetSystemLibrary.PrintString` "Ready" true true (struct :`R` 0.6625 :`G` 0.536639 :`A` 1.0))
      (`self.Move`)
      (`self.Emit No FX`)
      (set `self.clean` true)
      (`LightComponent.SetLightColor` (`self.PointLight`) (struct :`G` 1.0 :`A` 1.0) true)
      (clear `/Game/GameplayMechanics/Taser/Tasable_Component.On Tased` (`self.Tasable_Component`))
      (clear `/Game/GameplayMechanics/Taser/Tasable_Component.On Tasing` (`self.Tasable_Component`))
      (clear `/Game/GameplayMechanics/Taser/Tasable_Component.On Begin Tase` (`self.Tasable_Component`))
      (clear `/Game/GameplayMechanics/Taser/Tasable_Component.On End Tase` (`self.Tasable_Component`))
      (bind _asonline_session_gm (cast `/Game/Game/OnlineSession_GM` (`GameplayStatics.GetGameMode`)))
      (`/Game/Game/OnlineSession_GM.Update File in UI` _asonline_session_gm (`self.index`) "repaired")
      (bind _astasable_widget (cast `/Game/GameplayMechanics/Taser/Tasable_Widget` (`WidgetComponent.GetWidget` (`self.Widget`))))
      (`/Game/GameplayMechanics/Taser/Tasable_Widget.Should display widget` _astasable_widget false))))

(event `Reset Location`
  ;[1 1 1] Attach to cube
  (bind (_direction _alpha) (`Timeline|Reset` :!via `PlayFromStart`)
    (:`Update`
      (`SceneComponent.K2_SetRelativeLocation` (`self.Cube`) (`KismetMathLibrary.VLerp` (`SceneComponent.RelativeLocation` (`self.Cube`)) (0.0 0.0 0.0) _alpha) false false))))

(fn `get errors alpha`
  (returns (ReturnValue :type "Float (double-precision)"))
  (return (* (+ (`self.leftErrors`) (`self.rightErrors`)) 0.1)))

(fn `Swap Start & End`
  (locals (`vec Temp` :type "Vector Structure"))
  (set `local.vec Temp` (`SceneComponent.K2_GetComponentLocation` (`self.Start`)))
  (`SceneComponent.K2_SetWorldLocation` (`self.Start`) (`SceneComponent.K2_GetComponentLocation` (`self.End`)) false false)
  (`SceneComponent.K2_SetWorldLocation` (`self.End`) (`local.vec Temp`) false false))

(fn `UserConstructionScript`
  (`SceneComponent.K2_SetWorldLocation` (`self.Cube`) (`SceneComponent.K2_GetComponentLocation` (`self.Start`)) false false))